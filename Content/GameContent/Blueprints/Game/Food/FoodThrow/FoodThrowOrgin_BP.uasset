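; FoodThrowOrgin_BP is a food launcher that throws a steak from its location to a random throw spot shortly after play begins.
; It gathers all FoodThrowSpot_BP actors, then after a delay moves the picked spot from the available list to the taken list.
; It spawns a Steak_BP and lerps it to the spot using separate height and horizontal timelines at a shared play rate, forming an arc without physics.
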(event Custom|ThrowFoodServer
  (bind _output_get (Variables|Default|SetPickedThrowSpot (.OutItem (Utilities|Array|Random (Variables|Default|GetAvailableThrowSpots)))))
  (Utilities|Array|Add (Variables|Default|GetTakenThrowSpots) _output_get)
  (Utilities|Array|RemoveItem (Variables|Default|GetAvailableThrowSpots) _output_get)
  (CallFunction|ThrowFoodClient))

(event Custom|SetupServer
  (Utilities|FlowControl|Sequence
    (:then_0
      (bind _outactors (Actor|GetAllActorsOfClass "/Game/GameContent/Blueprints/Game/Food/FoodThrow/FoodThrowSpot_BP.FoodThrowSpot_BP_C"))
      (Variables|Default|SetAvailableThrowSpots _outactors))
    (:then_1
      (Utilities|FlowControl|Delay 3.0)
      (CallFunction|ThrowFoodServer))))

(event Custom|ThrowFoodClient
  (bind _self self)
  (bind _foodthrowplayrate (Variables|Default|GetFoodThrowPlayRate))
  (bind _pickedthrowspot (Variables|Default|GetPickedThrowSpot))
  (bind _returnvalue (Transformation|GetActorLocation _self))
  (bind _returnvalue_2 (Transformation|GetActorLocation _pickedthrowspot))
  (bind _returnvalue_3 (Game|SpawnActorfromClass "/Game/GameContent/Blueprints/Game/Food/FoodPickups/Steak_BP.Steak_BP_C" (Transformation|GetActorTransform) "Undefined" 0 0))
  (Variables|Default|SetFoodItem _returnvalue_3)
  (Utilities|FlowControl|Sequence
    (:then_0
      (Components|Timeline|SetPlayRate (Variables|Default|GetFoodArc_Z) _foodthrowplayrate)
      (bind _arcpath (Timeline|FoodArc_Z PlayFromStart)
        (:Update
          _)))
    (:then_1
      (Components|Timeline|SetPlayRate (Variables|Default|GetFoodArc_XY) _foodthrowplayrate)
      (bind _speed (Timeline|FoodArc_XY Play)
        (:Update
          _))))
  (Transformation|SetActorLocation (Variables|Default|GetFoodItem) (Math|Vector|MakeVector (.x (Math|Vector|Lerp(Vector) (Math|Vector|MakeVector (.x _returnvalue) (.y _returnvalue) 0.0) (Math|Vector|MakeVector (.x _returnvalue_2) (.y _returnvalue_2) 0.0) _speed)) (.y (Math|Vector|Lerp(Vector) (Math|Vector|MakeVector (.x _returnvalue) (.y _returnvalue) 0.0) (Math|Vector|MakeVector (.x _returnvalue_2) (.y _returnvalue_2) 0.0) _speed)) (.z (Math|Vector|Lerp(Vector) (Math|Vector|MakeVector 0.0 0.0 (.z _returnvalue)) (Math|Vector|MakeVector 0.0 0.0 (.z _returnvalue_2)) _arcpath))) false false))

(event EventBeginPlay
  (CallFunction|SetupServer))

(fn ConstructionScript)