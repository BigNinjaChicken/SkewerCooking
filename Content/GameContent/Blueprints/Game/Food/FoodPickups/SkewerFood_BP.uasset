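; SkewerFood_BP is a food pickup actor that can be placed on a skewer.
; It tracks whether it is on a skewer through a flag, set by the SetIsonSkewer event and read by GetIsOnSkewer.
; Getter functions expose its hit box, mesh and a fixed food size to other code.
; It has no active gameplay logic of its own, leaving skewering behavior to whatever calls it.
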(event EventBeginPlay)

(event Collision|EventActorBeginOverlap
  (params (OtherActor :type Actor%20Object%20Reference)))

(event EventTick
  (params (DeltaSeconds :type Float%20%28single-precision%29)))

(event EventSetIsonSkewer
  (params (OnSkewer :type Boolean))
  (Variables|Default|SetIsOnSkewer OnSkewer))

(fn ConstructionScript)

(fn GetFoodHitBoxComponent
  (return (Variables|Default|GetHitBox)))

(fn GetFoodMeshComponent
  (return (Variables|Default|GetMesh)))

(fn GetFoodSize
  (return 25.0))

(fn GetIsonSkewer
  (return (Variables|Default|GetIsOnSkewer)))